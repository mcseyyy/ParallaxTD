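; Base tower Blueprint that rises out of the ground when spawned and provides shared firing effects.
; BeginPlay sinks the model and enables Tick, which raises it over SpawnTime, then deactivates the spawning circle, plays a sound and calls the empty OnFinishedSpawning hook.
; OnFire plays the firing sound, while TriggerFireFlame activates a given flame particle with a yaw-only rotation computed from the tower and creep positions.
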(event `self.ReceiveBeginPlay`
  (bind _model (`self.Model`))
  (`KismetSystemLibrary.PrintString` null "Started Spwning")
  (`SceneComponent.K2_SetRelativeLocation` _model (- (`SceneComponent.RelativeLocation` _model) (0.0 0.0 650.0)) false)
  (`self.SetActorTickEnabled` true)
  (`KismetSystemLibrary.PrintString` null "Enabled Tick"))

(event `self.OnFire`
  (params (Target :type "BasicCreep Object Reference") (Projectile :type "BasicTowerProjectile Object Reference"))
  (`GameplayStatics.PlaySoundAtLocation` null (`self.OnFireSound`) (`self.SoundLocation`)))

(event `self.ReceiveActorBeginOverlap`
  (params (OtherActor :type "Actor Object Reference")))

(event `self.ReceiveTick`
  (params (DeltaSeconds :type "Float (single-precision)"))
  (bind _returnvalue (`KismetMathLibrary.FMin` 0.0 (+ (.z (`SceneComponent.RelativeLocation` (`self.Model`))) (* (/ DeltaSeconds (`self.SpawnTime`)) 650.0))))
  (if (not (`self.FinishedSpawning`))
    (`SceneComponent.K2_SetRelativeLocation` (`KismetMathLibrary.MakeVector` (.x (`SceneComponent.RelativeLocation` (`self.Model`))) (.y (`SceneComponent.RelativeLocation` (`self.Model`))) _returnvalue))
    (if (>= _returnvalue -0.01)
      (set `self.FinishedSpawning` true)
      (`ActorComponent.Deactivate` (`self.SpawningCircle`))
      (`GameplayStatics.PlaySoundAtLocation` null "/Game/Audio/Sounds-Music-Parallax/spawn/tower/tower02.tower02" (`self.SoundLocation`))
      (`self.OnFinishedSpawning`))))

(fn `Get FireFlame Rotation`
  (params (`Tower Location` :type "Object.Vector Structure" :default (0.0 0.0 0.0)) (`Target Location` :type "Object.Vector Structure" :default (0.0 0.0 0.0)))
  (returns (NewParam :type "Object.Rotator Structure"))
  (return (`KismetMathLibrary.MakeRot` 0.0 (`KismetMathLibrary.DegAtan2` (- (.y `Tower Location`) (.y `Target Location`)) (- (.x `Tower Location`) (.x `Target Location`))))))

(fn `OnFinishedSpawning`)

(fn `Trigger FireFlame`
  (params (`Particle Flame` :type "ParticleSystemComponent Object Reference") (`Creep Target` :type "BasicCreep Object Reference"))
  (bind _newparam (`self.Get FireFlame Rotation` (`self.K2_GetActorLocation`) (`self.K2_GetActorLocation` `Creep Target`)))
  (`SceneComponent.K2_SetWorldRotation` `Particle Flame` _newparam false)
  (`ActorComponent.Activate` `Particle Flame` false))

(fn `UserConstructionScript`
  (set `self.HeightStaticMesh` (.z (`SceneComponent.RelativeLocation` (`self.Model`)))))