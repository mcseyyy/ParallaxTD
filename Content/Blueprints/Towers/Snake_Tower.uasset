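; Snake tower Blueprint for a tower-defense game, extending a parent tower with an attack damage aura and a flame effect on firing.
; On BeginPlay it spawns an AttackDamageAura with a boosted damage multiplier and activates it on itself.
; Each shot runs the parent fire logic, then triggers the FireFlame particle toward the target creep.
; When spawning finishes it calls Activate with false.
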(event `self.ReceiveBeginPlay`
  (`parent.ReceiveBeginPlay`)
  (bind _returnvalue (`|SpawnActorFromClass` "/Game/Blueprints/Towers/Auras/AttackDamageAura.AttackDamageAura_C" (`KismetMathLibrary.MakeTransform` (0.0 0.0 0.0)) false 1.3))
  (`Aura.ActivateAura` _returnvalue self))

(event `self.OnFire`
  (params (Target :type "BasicCreep Object Reference") (Projectile :type "BasicTowerProjectile Object Reference"))
  (`parent.OnFire` Target Projectile)
  (`self.Trigger FireFlame` (`self.FireFlame`) Target))

(event `self.ReceiveActorBeginOverlap`
  (params (OtherActor :type "Actor Object Reference")))

(event `self.ReceiveTick`
  (params (DeltaSeconds :type "Float (single-precision)"))
  (`parent.ReceiveTick` DeltaSeconds))

(event `self.OnFinishedSpawning`
  (`ActorComponent.Activate` false))

(fn `UserConstructionScript`)