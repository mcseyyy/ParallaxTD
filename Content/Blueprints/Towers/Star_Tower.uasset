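; Star Tower is a tower Blueprint that gives its hits a chance to stun creeps.
; On hitting a creep, it rolls a random number against StunChance.
; On success it spawns a Slow debuff actor at full slow rate, sets its duration to StunDuration and applies it to the creep, so the stun reuses the slow effect.
; BeginPlay and Tick only call the parent class.
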(event `self.ReceiveBeginPlay`
  (`parent.ReceiveBeginPlay`))

(event `self.ReceiveActorBeginOverlap`
  (params (OtherActor :type "Actor Object Reference")))

(event `self.ReceiveTick`
  (params (DeltaSeconds :type "Float (single-precision)"))
  (`parent.ReceiveTick` DeltaSeconds))

(event `self.OnHitCreep`
  (params (Target :type "BasicCreep Object Reference"))
  (if (<= (`KismetMathLibrary.RandomFloatInRange` 0.0 1.0) (`self.Stun Chance`))
    (bind _returnvalue (`|SpawnActorFromClass` "/Game/Blueprints/Creeps/Debuffs/Slow.Slow_C" (`KismetMathLibrary.MakeTransform` (0.0 0.0 0.0)) false 1.0))
    (set `Debuff.Duration` (`self.Stun Duration`) _returnvalue)
    (`BasicCreep.ApplyDebuff` Target _returnvalue)))

(fn `UserConstructionScript`)