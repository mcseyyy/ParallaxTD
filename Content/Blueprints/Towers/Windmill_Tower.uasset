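; Windmill_Tower is a tower Blueprint that fires at creeps and applies an area slow on hit.
; It builds on a parent class, overriding OnFire to trigger the FireFlame effect toward the target creep.
; When a creep is hit, it spawns an Expslowsion actor with the tower's slow rate and duration, then activates its AoE with itself and that creep.
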(event `self.ReceiveBeginPlay`
  (`parent.ReceiveBeginPlay`))

(event `self.ReceiveActorBeginOverlap`
  (params (OtherActor :type "Actor Object Reference")))

(event `self.OnFire`
  (params (Target :type "BasicCreep Object Reference") (Projectile :type "BasicTowerProjectile Object Reference"))
  (`self.Trigger FireFlame` (`self.FireFlame`) Target))

(event `self.ReceiveTick`
  (params (DeltaSeconds :type "Float (single-precision)"))
  (`parent.ReceiveTick` DeltaSeconds))

(event `self.OnHitCreep`
  (params (Target :type "BasicCreep Object Reference"))
  (bind _returnvalue (`|SpawnActorFromClass` "/Game/Blueprints/Other/Expslowsion.Expslowsion_C" (`KismetMathLibrary.Conv_VectorToTransform` (0.0 0.0 0.0)) true (`self.Slow Rate`) (`self.Slow Duration`) self))
  (`AreaOfEffect.ActivateAoE` _returnvalue self Target))

(fn `UserConstructionScript`)