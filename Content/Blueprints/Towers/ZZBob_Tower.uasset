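; ZZBob_Tower is a tower Blueprint that sets off an explosion at its own position whenever it fires.
; OnFire runs the parent logic, then spawns an Explosion actor at the world origin, passing the tower's Damage and itself as instigator.
; The explosion is then activated at the tower's location, not the target's, with the tower as its source.
; BeginPlay and Tick only call the parent.
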(event `self.ReceiveBeginPlay`
  (`parent.ReceiveBeginPlay`))

(event `self.ReceiveActorBeginOverlap`
  (params (OtherActor :type "Actor Object Reference")))

(event `self.ReceiveTick`
  (params (DeltaSeconds :type "Float (single-precision)"))
  (`parent.ReceiveTick` DeltaSeconds))

(event `self.OnFire`
  (params (Target :type "BasicCreep Object Reference") (Projectile :type "BasicTowerProjectile Object Reference"))
  (`parent.OnFire` Target Projectile)
  (bind _returnvalue (`|SpawnActorFromClass` "/Game/Blueprints/Other/Explosion.Explosion_C" (`KismetMathLibrary.Conv_VectorToTransform` (0.0 0.0 0.0)) true (`self.Damage`) self))
  (`AreaOfEffect.ActivateAtLocation` _returnvalue self (`self.K2_GetActorLocation`)))

(fn `UserConstructionScript`)