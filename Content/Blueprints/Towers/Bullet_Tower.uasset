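; Tower Blueprint that deals area-of-effect damage when it hits a creep.
; On BeginPlay it moves the inherited Damage value into SplashDamage and zeroes Damage, leaving the damage to the explosion.
; OnHitCreep prints debug text, spawns an Explosion actor at the world origin with SplashDamage, then calls ActivateAoE with the tower and target.
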(event `self.ReceiveActorBeginOverlap`
  (params (OtherActor :type "Actor Object Reference")))

(event `self.ReceiveBeginPlay`
  (`parent.ReceiveBeginPlay`)
  (set `self.Splash Damage` (`self.Damage`))
  (set `self.Damage` 0))

(event `self.ReceiveTick`
  (params (DeltaSeconds :type "Float (single-precision)"))
  (`parent.ReceiveTick` DeltaSeconds))

(event `self.OnHitCreep`
  (params (Target :type "BasicCreep Object Reference"))
  (bind _splash_damage (`self.Splash Damage`))
  (`KismetSystemLibrary.PrintString` null "Inflicting Damage")
  (`KismetSystemLibrary.PrintString` null (`KismetStringLibrary.Conv_IntToString` _splash_damage))
  (bind _returnvalue (`|SpawnActorFromClass` "/Game/Blueprints/Other/Explosion.Explosion_C" (`KismetMathLibrary.Conv_VectorToTransform` (0.0 0.0 0.0)) true _splash_damage self))
  (`AreaOfEffect.ActivateAoE` _returnvalue self Target))

(fn `UserConstructionScript`)