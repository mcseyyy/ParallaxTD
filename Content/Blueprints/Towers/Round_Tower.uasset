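; Round_Tower is a tower Blueprint that extends a parent tower's firing and hit events.
; On fire, it runs the parent logic and triggers a fire flame particle toward the targeted creep.
; On hitting a creep, it rolls against CritChance and only on success inflicts Damage scaled by CritBonus, rounded up, without calling the parent hit handler.
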(event `self.ReceiveBeginPlay`
  (`parent.ReceiveBeginPlay`))

(event `self.OnFire`
  (params (Target :type "BasicCreep Object Reference") (Projectile :type "BasicTowerProjectile Object Reference"))
  (`parent.OnFire` Target Projectile)
  (`self.Trigger FireFlame` (`self.FireFlame`) Target))

(event `self.ReceiveActorBeginOverlap`
  (params (OtherActor :type "Actor Object Reference")))

(event `self.ReceiveTick`
  (params (DeltaSeconds :type "Float (single-precision)"))
  (`parent.ReceiveTick` DeltaSeconds))

(event `self.OnHitCreep`
  (params (Target :type "BasicCreep Object Reference"))
  (if (<= (`KismetMathLibrary.RandomFloatInRange` 0.0 1.0) (`self.Crit Chance`))
    (`BasicCreep.InflictDamage` Target (`KismetMathLibrary.FCeil` (* (`self.Damage`) (`self.Crit Bonus`))) self)))

(fn `UserConstructionScript`)