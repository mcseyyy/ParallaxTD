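; Tangerine Tower is a tower that periodically releases a stun explosion at its own location.
; Tick counts TimeToStun down from StunRate, then resets it and spawns a Stunsplosion actor with the tower's StunDuration.
; The actor spawns at the world origin, then ActivateAtLocation receives the tower as source and its location, leaving the stun effect to the Stunsplosion.
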(event `self.ReceiveBeginPlay`
  (`parent.ReceiveBeginPlay`)
  (set `self.Time To Stun` (`self.Stun Rate`)))

(event `self.ReceiveActorBeginOverlap`
  (params (OtherActor :type "Actor Object Reference")))

(event `self.ReceiveTick`
  (params (DeltaSeconds :type "Float (single-precision)"))
  (`parent.ReceiveTick` DeltaSeconds)
  (bind _output_get (set `self.Time To Stun` (- (`self.Time To Stun`) DeltaSeconds)))
  (if (<= _output_get 0.0)
    (set `self.Time To Stun` (`self.Stun Rate`))
    (bind _returnvalue (`|SpawnActorFromClass` "/Game/Blueprints/Other/Stunsplosion.Stunsplosion_C" (`KismetMathLibrary.MakeTransform` (0.0 0.0 0.0)) false (`self.Stun Duration`)))
    (`AreaOfEffect.ActivateAtLocation` _returnvalue self (`self.K2_GetActorLocation` self))))

(fn `UserConstructionScript`)