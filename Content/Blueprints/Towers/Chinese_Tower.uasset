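; Chinese tower, a child tower Blueprint that deals splash damage to creeps instead of direct-hit damage.
; On BeginPlay, after the parent runs, it moves Damage into SplashDamage and zeroes Damage.
; On each creep hit it spawns an Explosion at the world origin, assigns it SplashDamage, and calls ActivateAoE with itself and the target.
; Firing and Tick only forward to the parent.
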(event `self.OnFire`
  (params (Target :type "BasicCreep Object Reference") (Projectile :type "BasicTowerProjectile Object Reference"))
  (`parent.OnFire` Target Projectile))

(event `self.ReceiveActorBeginOverlap`
  (params (OtherActor :type "Actor Object Reference")))

(event `self.ReceiveTick`
  (params (DeltaSeconds :type "Float (single-precision)"))
  (`parent.ReceiveTick` DeltaSeconds))

(event `self.ReceiveBeginPlay`
  (`parent.ReceiveBeginPlay`)
  (`KismetSystemLibrary.PrintString` null "After parent")
  (set `self.Splash Damage` (`self.Damage`))
  (set `self.Damage` 0))

(event `self.OnHitCreep`
  (params (Target :type "BasicCreep Object Reference"))
  (bind _returnvalue (`|SpawnActorFromClass` "/Game/Blueprints/Other/Explosion.Explosion_C" (`KismetMathLibrary.Conv_VectorToTransform` (0.0 0.0 0.0)) true 0 self))
  (set `/Game/Blueprints/Other/Explosion.Damage` (`self.Splash Damage`) _returnvalue)
  (`AreaOfEffect.ActivateAoE` _returnvalue self Target))

(fn `UserConstructionScript`)