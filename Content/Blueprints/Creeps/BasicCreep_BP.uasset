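; Basic creep enemy Blueprint that handles sounds, health bar, death effects and stun state.
; BeginPlay polls until FinishedInit before playing its spawn sound, and Tick updates the health bar from current versus default HP.
; OnFinished and OnKilled play different sounds, then share an explosion sequence that hides model and bar and briefly sets Active.
; Stun functions toggle the AI controller's IsStunned blackboard key, while OnTakeDamage returns damage unchanged.
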(event `self.ReceiveBeginPlay`
  (if (`self.FinishedInit`) :!label _label
    (`GameplayStatics.PlaySoundAtLocation` null "/Game/Audio/Sounds-Music-Parallax/spawn/creep/creep01.creep01" (`self.SoundLocation`))
    (else
      (`KismetSystemLibrary.Delay` null 0.1)
      (goto _label))))

(event `self.OnFinished`
  ;[1 1 1] Activate Explosion on Creep Death
  (set `self.Active` true)
  (`GameplayStatics.PlaySoundAtLocation` null "/Game/Audio/Sounds-Music-Parallax/basereach/base01.base01" (`self.SoundLocation`))
  ;;[1 1 1] Explosion Stuff
  (`SceneComponent.SetHiddenInGame` (`self.Model`) true false :!label _label_2)
  (`SceneComponent.SetHiddenInGame` (`self.HP_Bar`) true false)
  (`ActorComponent.Activate` (`self.ExplosionComponent`) true)
  (`KismetSystemLibrary.Delay` null 0.5)
  (set `self.Active` false))

(event `self.OnKilled`
  (params (KillingTower :type "BasicTower Object Reference"))
  ;[1 1 1] Activate Explosion on Creep Death
  (set `self.Active` true)
  (`GameplayStatics.PlaySoundAtLocation` null "/Game/Audio/Sounds-Music-Parallax/creepdeath/death02.death02" (`self.SoundLocation`))
  (goto _label_2))

(event `self.ReceiveActorBeginOverlap`
  (params (OtherActor :type "Actor Object Reference")))

(event `self.ReceiveTick`
  (params (DeltaSeconds :type "Float (single-precision)"))
  ;[1 1 1] Update Health Bar
  (bind _returnvalue (`self.GetHP`))
  (bind _ashealth_bar_progress_bar (cast `/Game/Blueprints/Creeps/HealthBars/HealthBar_progressBar` (`WidgetComponent.GetUserWidgetObject`)))
  (`ProgressBar.SetPercent` (`/Game/Blueprints/Creeps/HealthBars/HealthBar_progressBar.ProgressBar_31` _ashealth_bar_progress_bar) (/ (`KismetMathLibrary.Conv_IntToDouble` _returnvalue) (`KismetMathLibrary.Conv_IntToDouble` (`self.DefaultHP`)))))

(fn `OnTakeDamage`
  (params (DamageReceived :type Integer))
  (returns (Damage :type Integer))
  (return DamageReceived))

(fn `StartStun`
  (bind _returnvalue (`AIBlueprintHelperLibrary.GetAIController` self))
  (bind _asbasic_creep_aicontroller (cast `BasicCreepAIController` _returnvalue))
  (`BlackboardComponent.SetValueAsBool` (`AIBlueprintHelperLibrary.GetBlackboard` _asbasic_creep_aicontroller) "IsStunned" true))

(fn `StopStun`
  (bind _returnvalue (`AIBlueprintHelperLibrary.GetAIController` self))
  (bind _asbasic_creep_aicontroller (cast `BasicCreepAIController` _returnvalue))
  (`BlackboardComponent.SetValueAsBool` (`AIBlueprintHelperLibrary.GetBlackboard` _asbasic_creep_aicontroller) "IsStunned" false))

(fn `UserConstructionScript`)