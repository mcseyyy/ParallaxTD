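; Mushroom creep Blueprint that applies negative damage to a team when it finishes, apparently restoring one point to its owner's side.
; On the finished event it casts the game mode to PlayGameMode, derives the team index from OwnerID divided by MaxSlots, and calls InflictDamage with minus one on that team.
; BeginPlay and Tick only defer to the parent class.
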(event `self.ReceiveBeginPlay`
  (`parent.ReceiveBeginPlay`))

(event `self.ReceiveActorBeginOverlap`
  (params (OtherActor :type "Actor Object Reference")))

(event `self.ReceiveTick`
  (params (DeltaSeconds :type "Float (single-precision)"))
  (`parent.ReceiveTick` DeltaSeconds))

(event `self.OnFinished`
  (bind _asplay_game_mode (cast `PlayGameMode` (`GameplayStatics.GetGameMode` null)))
  (bind _returnvalue (`PlayGameMode.GetTeam` _asplay_game_mode (/ (`self.OwnerID`) (`PlayGameMode.MaxSlots` _asplay_game_mode))))
  (`Battlefield.InflictDamage` _returnvalue -1))

(fn `UserConstructionScript`)