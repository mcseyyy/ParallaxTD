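; Tired_Creep is a creep variant that has a chance to revive once when killed.
; On its killed event, a random roll against ReviveChance sets it active and alive again at half its default HP.
; A HasRevived flag blocks any further revival, and the killed event makes no parent call.
; BeginPlay and Tick only forward to the parent class.
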(event `self.ReceiveBeginPlay`
  (`parent.ReceiveBeginPlay`))

(event `self.ReceiveActorBeginOverlap`
  (params (OtherActor :type "Actor Object Reference")))

(event `self.ReceiveTick`
  (params (DeltaSeconds :type "Float (single-precision)"))
  (`parent.ReceiveTick` DeltaSeconds))

(event `self.OnKilled`
  (params (KillingTower :type "BasicTower Object Reference"))
  (if (and (not (`self.Has Revived`)) (<= (`KismetMathLibrary.RandomFloatInRange` 0.0 1.0) (`self.Revive Chance`)))
    (set `self.Has Revived` true)
    (set `self.Active` true)
    (set `self.Alive` true)
    (set `self.CurrentHP` (/ (`self.DefaultHP`) 2))))

(fn `UserConstructionScript`)