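; Lobby game mode that drives the on-screen lobby display for a six-slot, blue-versus-red team match.
; On BeginPlay it creates the LobbyDisplay widget, sets team names and colours, and marks every slot empty, using -1 as the no-player ready state.
; Join, leave, ready and swap events update slot names, colours or ready states from Players, ReadySet or event arguments.
; Game start removes the widget.
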(event `self.ReceiveBeginPlay`
  (bind _returnvalue (`|CreateWidget` "/Game/Widgets/LobbyDisplay.LobbyDisplay_C"))
  (set `/Game/Widgets/LobbyDisplay.Team 1 Name` "BLUE  TEAM" _returnvalue)
  (set `/Game/Widgets/LobbyDisplay.Team 1 Colour` (`KismetMathLibrary.MakeColor` 0.0 0.0 1.0 1.0) _returnvalue)
  (set `/Game/Widgets/LobbyDisplay.Team 2 Name` "RED  TEAM" _returnvalue)
  (set `/Game/Widgets/LobbyDisplay.Team 2 Colour` (`KismetMathLibrary.MakeColor` 1.0 0.0 0.0 1.0) _returnvalue)
  (for _index (range 6)
    (`/Game/Widgets/LobbyDisplay.SetPlayerName` _returnvalue _index "Empty")
    (`/Game/Widgets/LobbyDisplay.SetPlayerReady` _returnvalue _index -1))
  (`UserWidget.AddToViewport` _returnvalue 0)
  (set `self.LobbyDisplay` _returnvalue))

(event `self.ReceiveTick`
  (params (DeltaSeconds :type "Float (single-precision)")))

(event `self.OnPlayerJoin`
  (params (PlayerID :type Integer))
  (bind _lobbydisplay (`self.LobbyDisplay`))
  (bind (_name _colour) (break `PlayerConnectionHandler.PlayerData` (`KismetArrayLibrary.Array_Get` (`self.Players`) PlayerID)))
  (`/Game/Widgets/LobbyDisplay.SetPlayerColour` _lobbydisplay PlayerID (`KismetMathLibrary.Conv_ColorToLinearColor` _colour))
  (`/Game/Widgets/LobbyDisplay.SetPlayerName` _lobbydisplay PlayerID _name))

(event `self.OnGameStart`
  (`Widget.RemoveFromParent` (`self.LobbyDisplay`)))

(event `self.OnPlayerLeave`
  (params (PlayerID :type Integer))
  (bind _lobbydisplay (`self.LobbyDisplay`))
  (`/Game/Widgets/LobbyDisplay.SetPlayerName` _lobbydisplay PlayerID "Empty")
  (`/Game/Widgets/LobbyDisplay.SetPlayerReady` _lobbydisplay PlayerID -1))

(event `self.OnPlayerSetReady`
  (params (PlayerID :type Integer) (Ready :type Boolean))
  (`/Game/Widgets/LobbyDisplay.SetPlayerReady` (`self.LobbyDisplay`) PlayerID (`KismetMathLibrary.Conv_BoolToInt` Ready)))

(event `self.OnPlayerSwap`
  (params (PlayerA :type Integer) (PlayerB :type Integer))
  (bind _players (`self.Players`))
  (bind _readyset (`self.ReadySet`))
  (bind _lobbydisplay (`self.LobbyDisplay`))
  (bind (_name _colour) (break `PlayerConnectionHandler.PlayerData` (`KismetArrayLibrary.Array_Get` _players PlayerB)))
  (bind (_name_2 _colour_2) (break `PlayerConnectionHandler.PlayerData` (`KismetArrayLibrary.Array_Get` _players PlayerA)))
  (`/Game/Widgets/LobbyDisplay.SetPlayerColour` _lobbydisplay PlayerB (`KismetMathLibrary.Conv_ColorToLinearColor` _colour_2))
  (`/Game/Widgets/LobbyDisplay.SetPlayerName` _lobbydisplay PlayerB _name_2)
  (`/Game/Widgets/LobbyDisplay.SetPlayerReady` _lobbydisplay PlayerB (`KismetMathLibrary.Conv_BoolToInt` (`KismetArrayLibrary.Array_Get` _readyset PlayerB)))
  (`/Game/Widgets/LobbyDisplay.SetPlayerColour` _lobbydisplay PlayerA (`KismetMathLibrary.Conv_ColorToLinearColor` _colour))
  (`/Game/Widgets/LobbyDisplay.SetPlayerName` _lobbydisplay PlayerA _name)
  (`/Game/Widgets/LobbyDisplay.SetPlayerReady` _lobbydisplay PlayerA (`KismetMathLibrary.Conv_BoolToInt` (`KismetArrayLibrary.Array_Get` _readyset PlayerA))))

(fn `UserConstructionScript`)