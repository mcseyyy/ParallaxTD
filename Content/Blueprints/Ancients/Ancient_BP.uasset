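; Ancient base structure that shows progressive fire and smoke as its health drops and can be blown apart.
; The construction script gathers the fire and smoke components into an ordered array.
; SetFire activates effects whose evenly spaced index threshold exceeds the given HP percentage, starting from the array's end and never deactivating them.
; ExplodeBase applies damage with an upward impulse at the actor's location; the event graph is unused.
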(event `self.ReceiveBeginPlay`)

(event `self.ReceiveActorBeginOverlap`
  (params (OtherActor :type "Actor Object Reference")))

(event `self.ReceiveTick`
  (params (DeltaSeconds :type "Float (single-precision)")))

(fn `ExplodeBase`
  (`DestructibleComponent.ApplyDamage` 10.0 (`self.K2_GetActorLocation`) (`KismetMathLibrary.MakeVector` 0.0 0.0 10.0) 10.0))

(fn `SetFire`
  (params (HP_Percentage :type "Float (double-precision)" :default 0.0))
  (bind _returnvalue (`KismetArrayLibrary.Array_LastIndex` (`self.Fire`)))
  (for _index (range (+ _returnvalue 1))
    (if (> (* (`KismetMathLibrary.Conv_IntToDouble` (+ _index 1)) (/ 1.0 (`KismetMathLibrary.Conv_IntToDouble` (+ _returnvalue 2)))) HP_Percentage)
      (bind _item (`KismetArrayLibrary.Array_Get` (`self.Fire`) _index))
      (cast `ParticleSystemComponent` _item
        (:`then`
          (`ActorComponent.Activate` _item false))
        (:`CastFailed`
          (`KismetSystemLibrary.PrintString` "Hello"))))))

(fn `UserConstructionScript`
  (bind _fire (`self.Fire`))
  (`KismetArrayLibrary.Array_Resize` _fire)
  (`KismetArrayLibrary.Array_Add` _fire (`self.Fire0`))
  (`KismetArrayLibrary.Array_Add` _fire (`self.Fire1`))
  (`KismetArrayLibrary.Array_Add` _fire (`self.Fire2`))
  (`KismetArrayLibrary.Array_Add` _fire (`self.Fire3`))
  (`KismetArrayLibrary.Array_Add` _fire (`self.Smoke0`))
  (`KismetArrayLibrary.Array_Add` _fire (`self.Fire4`))
  (`KismetArrayLibrary.Array_Add` _fire (`self.Fire5`))
  (`KismetArrayLibrary.Array_Add` _fire (`self.Smoke1`))
  (`KismetArrayLibrary.Array_Add` _fire (`self.Fire6`))
  (`KismetArrayLibrary.Array_Add` _fire (`self.Smoke2`))
  (`KismetArrayLibrary.Array_Resize` _fire 10))